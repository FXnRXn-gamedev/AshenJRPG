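; BP_FieldPlayer is the player-controlled pawn for the field part of the game.
; It adds the Enhanced Input mapping context on possession and moves along world X and Y from IA_Move.
; On BeginPlay it messages the player controller through interfaces to create the field widget and plays the screen-open transition.
; StoreFieldPositionOnInstance saves its transform and current level name to the GameInstance through interface messages.
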(event Input|EnhancedActionEvents|EnhancedInputActionIA_Move
  (params (ActionValue :type Vector%202D%20Structure) (ElapsedSeconds :type Float%20%28double-precision%29) (TriggeredSeconds :type Float%20%28double-precision%29) (InputAction :type Input%20Action%20Object%20Reference :default "/Game/_PROJECT_/Inputs/Field/Actions/IA_Move.IA_Move"))
  (bind (_x _y) (Math|Vector2D|BreakVector2D ActionValue))
  (Pawn|Input|AddMovementInput "1.000000,0.000000,0.000000" _x false)
  (Pawn|Input|AddMovementInput "0.000000,1.000000,0.000000" _y false))

(event EventBeginPlay
  (|CallParentFunction)
  ;[0.15 0.15 0.15 0.5] Init Field Widget
  (Class|BPIUIControl|IInitWidgetField(Message) (Game|GetPlayerController 0))
  ;[0.15 0.15 0.15 0.5 55] Transition Anim Open
  (bind _widgetbattle (Class|BPIUIControl|IGetWidgetBattle(Message) (Game|GetPlayerController 0)))
  (bind _wbp_transition (Variables|/Game/_PROJECT_/Blueprints/Widgets/WBP_Battle.WBP_Battle_C|GetWBP_Transition _widgetbattle)
    (:then
      (Default|PlayScreenOpenAnim _wbp_transition))
    (:else)))

(event Collision|EventActorBeginOverlap
  (params (OtherActor :type Actor%20Object%20Reference))
  (|CallParentFunction OtherActor) ; This node is disabled and will not be called.\nDrag off pins to build functionality.
)

(event EventTick
  (params (DeltaSeconds :type Float%20%28single-precision%29))
  (|CallParentFunction DeltaSeconds) ; This node is disabled and will not be called.\nDrag off pins to build functionality.
)

(event EventPossessed
  (params (NewController :type Controller%20Object%20Reference))
  (|CallParentFunction NewController)
  ;[0.15 0.15 0.15 0.5] Cast To PlayerController
  (bind _asplayer_controller (Utilities|Casting|CastToPlayerController (Pawn|GetController)))
  ;[0.15 0.15 0.15 0.5] Enhanced Input System
  (Input|AddMappingContext (PlayerController|LocalPlayerSubsystems|GetEnhancedInputLocalPlayerSubsystem _asplayer_controller) (Variables|Input|GetMapping%20Context) 0 "(bIgnoreAllPressedKeysUntilRelease=True,bForceImmediately=False,bNotifyUserSettings=False)"))

(fn ConstructionScript
  (|CallParentFunction))

(fn StoreFieldPositiononInstance
  ;[0.15 0.15 0.15 0.5] Store Field Transform
  (Class|BPIInstance|IStoreFieldPosition(Message) (Game|GetGameInstance) (Transformation|GetActorTransform))
  ;[0.15 0.15 0.15 0.5] Store Level Name
  (bind _returnvalue (Game|GetCurrentLevelName true))
  (Class|BPIInstance|IFieldLevelName(Message) (Game|GetGameInstance) _returnvalue))