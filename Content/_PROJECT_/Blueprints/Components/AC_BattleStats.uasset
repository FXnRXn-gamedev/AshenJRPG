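; Battle stats component that holds a character's attributes and HP/MP state, seeded from the owner's battle data.
; ReceiveBattleEffect turns a skill's calculated power into damage through defense reduction and a defending multiplier, rounded to at least 1.
; It clamps HP at zero, updates the health widget and shows combat numbers with critical styling.
; Zero HP flags knockout and calls DepletedHealth on the owner; otherwise the character shakes.
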(event EventBeginPlay)

(event EventTick
  (params (DeltaSeconds :type Float%20%28single-precision%29)))

(fn Initialize
  (params (OwningBattleChar :type BP%20Battle%20Char%20Base%20Object%20Reference))
  (Variables|Default|SetOwningBattleChar OwningBattleChar)
  (bind _owningbattlechar (Variables|Default|GetOwningBattleChar)
    (:then
      (bind _output_get (Variables|Default|SetAttributes (Variables|/Game/_PROJECT_/Data/DataAssets/BattleCharData/PDA_BattleCharData.PDA_BattleCharData_C|GetInitialAttributes (Variables|/Game/_PROJECT_/Blueprints/Battle/BattleChars/BP_BattleChar_Base.BP_BattleChar_Base_C|GetBattleCharData _owningbattlechar))))
      (Utilities|Struct|SetmembersinS_CharState (Variables|Default|GetState) (.MaxHP (Utilities|Struct|BreakS_CharAttributes _output_get)) (.MaxMP (Utilities|Struct|BreakS_CharAttributes _output_get))))
    (:else)))

(fn ReceiveBattleEffect
  (params (InstigatorStats :type AC%20Battle%20Stats%20Object%20Reference) (SkillData :type PDA%20Skill%20Data%20Object%20Reference))
  (Utilities|FlowControl|Sequence
    (:then_0
      ;[0.15 0.15 0.15 0.5 32] CurrentHP = [State] HP - [PDA_SkillData] CalculatedAttackPower(f)
      (bind (_calculatedpower _wascritical) (Default|GetCalculatedPower SkillData InstigatorStats))
      (LocalVariables|SetIsCritical _wascritical)
      ;;[0.15 0.15 0.15 0.5] After Using Defense
      (bind _damage (CallFunction|DamageAfterDefense _calculatedpower (Variables|/Game/_PROJECT_/Data/DataAssets/SkillData/PDA_SkillData.PDA_SkillData_C|GetIsPhysical SkillData)))
      ;;[0.15 0.15 0.15 0.5] Final Damage Value
      (LocalVariables|SetFinalPowerValue (Math|Conversions|ToFloat(Integer) (Math|Integer|Max(Integer) (Math|Float|Round _damage) 1)))
      (bind _structout (Utilities|Struct|SetmembersinS_CharState (Variables|Default|GetState) (Math|Float|Max(Float) (- (Utilities|Struct|BreakS_CharState (Variables|Default|GetState)) (LocalVariables|GetFinalPowerValue)) 0.0)))
      ;[0.15 0.15 0.15 0.5 32] Update Widget  HP
      (bind _widgethealthmana (Variables|/Game/_PROJECT_/Blueprints/Battle/BattleChars/BP_BattleChar_Base.BP_BattleChar_Base_C|GetWidgetHealthMana (Variables|Default|GetOwningBattleChar))
        (:then
          (Default|UpdateHPWidget _widgethealthmana (Utilities|Struct|BreakS_CharState _structout) (Utilities|Struct|BreakS_CharAttributes (Variables|Default|GetAttributes))))
        (:else)))
    (:then_1
      ;[0.15 0.15 0.15 0.5 32] Show Damage Widget Text
      (Default|ShowText (Variables|/Game/_PROJECT_/Blueprints/Battle/BattleChars/BP_BattleChar_Base.BP_BattleChar_Base_C|GetWidgetCombatNumber (Variables|Default|GetOwningBattleChar)) (LocalVariables|GetFinalPowerValue) (select (LocalVariables|GetIsCritical) "NewEnumerator1" "NewEnumerator0")))
    (:then_2
      ;[0.15 0.15 0.15 0.5 32] Knockdown condition (if hp 0)
      (if (<= (Utilities|Struct|BreakS_CharState (Variables|Default|GetState)) 0.0)
        ;[0.15 0.15 0.15 0.5 32] Knockout true
        (Utilities|Struct|SetmembersinS_CharState (Variables|Default|GetState) true)
        ;[0.15 0.15 0.15 0.5] Call DepletedHealth in BattleChar_Base
        (Default|DepletedHealth (Variables|Default|GetOwningBattleChar))
        (else
          ;[0.15 0.15 0.15 0.5 32] Shake Effect (Only hp != 0)
          (Default|StartShake (Variables|/Game/_PROJECT_/Blueprints/Battle/BattleChars/BP_BattleChar_Base.BP_BattleChar_Base_C|GetAC_Shaker (Variables|Default|GetOwningBattleChar))))))))

(fn DamageAfterDefense
  (params (IncomingDamage :type Float%20%28double-precision%29) (IsPhysical :type Boolean))
  (return (* (- IncomingDamage (|DamageReduction)) (select (Variables|/Game/_PROJECT_/Blueprints/Battle/BattleChars/BP_BattleChar_Base.BP_BattleChar_Base_C|GetIsDefending (Variables|Default|GetOwningBattleChar)) (Variables|/Game/_PROJECT_/Data/DataAssets/GlobalVariables/PDA_GlobalVariables.PDA_GlobalVariables_C|GetDefendMultiplier (CallFunction|GetGlobalVariables)) 1.0))))