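; AC_Shaker is a component that shakes a scene component, supplied through Initialize, back and forth along its relative X axis.
; StartShake runs a looping interval timer, apparently driving ShakeOnce, which uses a FlipFlop to alternate between positive and negative X offsets.
; A retriggerable delay then calls EndShake, which clears the timer and resets relative X to zero rather than the original value, preserving Y and Z.
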(event Custom|ShakeOnce
  (bind _shaketransx (Variables|ComponentProperties|GetShakeTransX))
  (bind _comptoshake (Variables|ComponentProperties|GetCompToShake))
  (bind _relativelocation (Variables|/Script/Engine.SceneComponent|GetRelativeLocation _comptoshake))
  (bind _isa (Utilities|FlowControl|FlipFlop)
    (:A
      _)
    (:B
      _))
  ;[0.15 0.15 0.15 0.5] Shake Functionality
  (Transformation|SetRelativeLocation (Variables|ComponentProperties|GetCompToShake) (Math|Vector|MakeVector (Math|Float|SelectFloat _shaketransx (* _shaketransx -1.0) _isa) (.y _relativelocation) (.z _relativelocation)) false false))

(event Custom|StartShake
  ;[0.15 0.15 0.15 0.5] Create Shake Event and Assign to Var - End shake after delay
  (bind _returnvalue (Utilities|Time|SetTimerbyEvent (EventDispatchers|CreateEvent :!event Custom|ShakeOnce) (Variables|ComponentProperties|GetShakeInterval) true))
  (Variables|ComponentProperties|SetShakeHandle _returnvalue)
  (Utilities|FlowControl|RetriggerableDelay (Variables|ComponentProperties|GetShakeDuration))
  (CallFunction|EndShake))

(event Custom|EndShake
  (bind _comptoshake (Variables|ComponentProperties|GetCompToShake))
  (bind _relativelocation (Variables|/Script/Engine.SceneComponent|GetRelativeLocation _comptoshake))
  ;[0.15 0.15 0.15 0.5] End Shake Event By Clear time event
  (Utilities|Time|ClearandInvalidateTimerbyHandle (Variables|ComponentProperties|GetShakeHandle))
  ;[0.15 0.15 0.15 0.5] Reset conponent position
  (Transformation|SetRelativeLocation (Variables|ComponentProperties|GetCompToShake) (Math|Vector|MakeVector 0.0 (.y _relativelocation) (.z _relativelocation)) false false))

(event EventBeginPlay)

(fn Initialize
  (params (CompToShake :type Scene%20Component%20Object%20Reference))
  (Variables|ComponentProperties|SetCompToShake CompToShake))