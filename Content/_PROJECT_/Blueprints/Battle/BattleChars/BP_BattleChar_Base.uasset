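; BP_BattleChar_Base is the base battle character for party members and enemies in a turn-based battle, using an animated sprite.
; Attacks play skill animations, or a timeline jump as fallback, and report back to BattleManagerBP.
; ACBattleStats handles mana, damage and healing, with effects routed by target group and Niagara VFX.
; At zero HP, party members switch to Downed while enemies play a knockback and hide; targeting pulses the sprite material.
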(event Custom|PlayAttackAnim
  (params (SkillData :type PDA%20Skill%20Data%20Object%20Reference))
  (bind _spawnedlocation (Variables|Default|GetSpawnedLocation))
  ;[0.15 0.15 0.15 0.5] Get Animation from data(Chek validity) and Play Attack Animation
  ;;[0.15 0.15 0.15 0.5] Get Appropriate Attack Anim
  (bind _animation (CallFunction|PickSkillAnim SkillData))
  (Utilities|IsValid _animation
    (:Is%20Valid
      (|PlayAnimationOverridewithCallbacks (Variables|/Script/PaperZD.PaperZDAnimationComponent|GetAnimInstance (Variables|Default|GetAnimationComponent)) _animation "DefaultSlot" 1.0 0.0
        (:then
          ;[0.15 0.15 0.15 0.5] Cost Mana
          (Default|UpdateMana (Variables|Default|GetAC_BattleStats) (* (Variables|/Game/_PROJECT_/Data/DataAssets/SkillData/PDA_SkillData.PDA_SkillData_C|GetManaCost SkillData) -1.0)))
        (:OnCompleted
          ;[0.15 0.15 0.15 0.5] Delay
          (Utilities|FlowControl|RetriggerableDelay (Variables|/Game/_PROJECT_/Data/DataAssets/GlobalVariables/PDA_GlobalVariables.PDA_GlobalVariables_C|GetDelayAfterAttackAnim (CallFunction|GetGlobalVariables)) :!label _label)
          ;[0.15 0.15 0.15 0.5] Attack Finish - Move back to Init Location
          (bind _battlemanagerbp (Variables|Default|GetBattleManagerBP)
            (:then
              (Default|MoveBacktoInitLocation _battlemanagerbp))
            (:else)))
        (:OnCancelled
          (goto _label))))
    (:Is%20Not%20Valid
      ;[0.15 0.15 0.15 0.5] Play DoubleJump
      (Components|Timeline|SetPlayRate (Variables|Default|GetAnimDoubleJump) (Variables|Jump|GetJumpPlayRate))
      (bind _alpha (Timeline|AnimDoubleJump PlayFromStart)
        (:Update
          (Transformation|SetActorLocation (Math|Vector|MakeVector (.x _spawnedlocation) (.y _spawnedlocation) (+ (.z _spawnedlocation) (* _alpha (Variables|Jump|GetJumpHeight)))) false false))
        (:Finished
          ;[0.15 0.15 0.15 0.5] Call Finished timeline Attack in BattleManager
          (bind _battlemanagerbp_2 (Variables|Default|GetBattleManagerBP)
            (:then
              (Default|FinishedTimelineAttackAnim _battlemanagerbp_2))
            (:else)))))))

(event Custom|PlayKnockoutAnim
  ;[0.15 0.15 0.15 0.5] Knockout Anim Functionality
  (Components|Timeline|SetPlayRate (Variables|Default|GetAnimKnockout) (Variables|Knockout|GetKnockoutAnimPlayRate))
  (bind _alpha (Timeline|AnimKnockout PlayFromStart)
    (:Update
      (Transformation|SetActorLocation (Math|Vector|Lerp(Vector) (Variables|Default|GetSpawnedLocation) (+ (Variables|Default|GetSpawnedLocation) (Variables|Knockout|GetKnockoutOffset)) _alpha) false false))
    (:Finished
      ;[0.15 0.15 0.15 0.5] After finish knockoutAnim, Hidden Gameobject
      (Rendering|SetActorHiddenInGame true))))

(event EventBeginPlay
  (Utilities|FlowControl|Sequence
    (:then_0
      ;[0.15 0.15 0.15 0.5] Save Charcter Location
      (Variables|Default|SetSpawnedLocation (Transformation|GetActorLocation))
      ;[0.15 0.15 0.15 0.5] Get Reffereence of ActionPointer Widget
      (|InitWidgetPointer)
      ;[0.15 0.15 0.15 0.5] Get Refference of CombatText Widget
      (|InitWidgetCombatText))
    (:then_1
      ;[0.15 0.15 0.15 0.5] Shaker Component Initialization
      (Default|Initialize (Variables|Default|GetAC_Shaker) (Variables|Default|GetSprite))
      ;[0.15 0.15 0.15 0.5] BattleStats Component Initialization
      (Default|Initialize (Variables|Default|GetAC_BattleStats) self))
    (:then_2
      ;[0.15 0.15 0.15 0.5] Material
      (bind _returnvalue (Rendering|Material|CreateDynamicMaterialInstance (Variables|Default|GetSprite) 0 0 "None" :!class /Script/Engine.PrimitiveComponent))
      (Variables|Material|SetDynamicSpriteMat _returnvalue))))

(fn ConstructionScript)

(fn HideBattlePortraitWidget
  (bind _widgetpotrait (Variables|Widget|GetWidgetPotrait)
    (:then
      (Default|SetPortraitVisibility _widgetpotrait "Collapsed" false false)
      ;[0.15 0.15 0.15 0.5] Set Null after Hide
      (Variables|Widget|SetWidgetPotrait 0))
    (:else)))

(fn AssignBattleHealthManaWidget
  (params (WidgetHealthMana :type WBP%20Battle%20Health%20Mana%20Object%20Reference))
  (bind _ac_battlestats (Variables|Default|GetAC_BattleStats))
  (bind _ac_battlestats_2 (Variables|Default|GetAC_BattleStats))
  (bind _battlechardata (Variables|Default|GetBattleCharData))
  (bind _attributes (Variables|/Game/_PROJECT_/Blueprints/Components/AC_BattleStats.AC_BattleStats_C|GetAttributes _ac_battlestats_2))
  (bind _state (Variables|/Game/_PROJECT_/Blueprints/Components/AC_BattleStats.AC_BattleStats_C|GetState _ac_battlestats))
  (bind (_hp _mp) (Utilities|Struct|BreakS_CharState _state))
  (bind (_maxhp _maxmp) (Utilities|Struct|BreakS_CharAttributes _attributes))
  (Variables|Widget|SetWidgetHealthMana WidgetHealthMana)
  (bind _widgethealthmana (Variables|Widget|GetWidgetHealthMana)
    (:then
      (Default|ActivateBattleStat _widgethealthmana (Variables|/Game/_PROJECT_/Data/DataAssets/BattleCharData/PDA_BattleCharData.PDA_BattleCharData_C|GetPortfolioImage _battlechardata) (Variables|/Game/_PROJECT_/Data/DataAssets/BattleCharData/PDA_BattleCharData.PDA_BattleCharData_C|GetDisplayName _battlechardata) _maxhp _hp _maxmp _mp))
    (:else)))

(fn SetPointerVisibility
  (params (SetVisibile :type Boolean))
  (if SetVisibile
    ;[0.15 0.15 0.15 0.5] Target Pointer Visibility
    (Default|ShowPointer (Variables|Widget|GetWidgetTargetPointerRef))
    ;[0.15 0.15 0.15 0.5] Change Param for FlashMaterial
    (Rendering|Material|SetScalarParameterValue (Variables|Material|GetDynamicSpriteMat) "IsPulsing" 1.0 :!class /Script/Engine.MaterialInstanceDynamic)
    (else
      (Default|HidePointer (Variables|Widget|GetWidgetTargetPointerRef))
      (Rendering|Material|SetScalarParameterValue (Variables|Material|GetDynamicSpriteMat) "IsPulsing" 0.0 :!class /Script/Engine.MaterialInstanceDynamic))))

(fn RecieveBattleEffect
  (params (InstigatorStats :type AC%20Battle%20Stats%20Object%20Reference) (CurrentSkillData :type PDA%20Skill%20Data%20Object%20Reference))
  ;[0.15 0.15 0.15 0.5] VFX Effect
  (Niagara|SpawnSystematLocation (Variables|/Game/_PROJECT_/Data/DataAssets/SkillData/PDA_SkillData.PDA_SkillData_C|GetParticleEffect CurrentSkillData) (+ (Transformation|GetWorldLocation (Utilities|Select :Index (Variables|/Game/_PROJECT_/Data/DataAssets/SkillData/PDA_SkillData.PDA_SkillData_C|GetParticleLocation CurrentSkillData) :NewEnumerator0 (Variables|Default|GetLoc_Head) :NewEnumerator1 (Variables|Default|GetLoc_Middle) :NewEnumerator2 (Variables|Default|GetLoc_Feet))) (Variables|/Game/_PROJECT_/Data/DataAssets/SkillData/PDA_SkillData.PDA_SkillData_C|GetParticleLocationOffset CurrentSkillData)) "0, 0, 0" "1.000000,1.000000,1.000000" true true "AutoRelease")
  (switch Utilities|FlowControl|Switch|SwitchonE_TargetGroup (Variables|/Game/_PROJECT_/Data/DataAssets/SkillData/PDA_SkillData.PDA_SkillData_C|GetTargetGroup CurrentSkillData)
    (:NewEnumerator0
      ;[0.15 0.15 0.15 0.5] Damage Effect
      (Default|ReceiveDamageEffect (Variables|Default|GetAC_BattleStats) InstigatorStats CurrentSkillData))
    (:NewEnumerator1
      ;[0.15 0.15 0.15 0.5] Heal Effect
      (Default|ReceiveHealEffect (Variables|Default|GetAC_BattleStats) InstigatorStats CurrentSkillData))))

(fn ExecuteBattleEffect
  ;[0.15 0.15 0.15 0.5] It call BattleManager - Get Target and Apply effect to Base char class [It will trigger from notify]
  (bind _battlemanagerbp (Variables|Default|GetBattleManagerBP)
    (:then
      (Default|ApplyBattleEffect _battlemanagerbp (Variables|Default|GetAC_BattleStats)))
    (:else)))

(fn SetDefending
  (params (SetActive :type Boolean))
  (Variables|Defend|SetIsDefending SetActive))

(fn DepletedHealth
  (Utilities|FlowControl|Sequence
    (:then_0
      ;[0.15 0.15 0.15 0.5] Pass character to remove
      (bind _battlemanagerbp (Variables|Default|GetBattleManagerBP)
        (:then
          (Default|UpdateTeamAlive _battlemanagerbp self)
          ;[0.15 0.15 0.15 0.5] Widget : Set Protrait Visibility that remove from turnorder
          (bind _widgetpotrait (Variables|Widget|GetWidgetPotrait)
            (:then
              (Default|SetPortraitVisibility _widgetpotrait "Visible" false true))
            (:else)))
        (:else)))
    (:then_1
      ;[0.15 0.15 0.15 0.5] Check is it Party member or Enemy
      (if (Variables|Default|GetIsPartyMember)
        ;[0.15 0.15 0.15 0.5] Depleted Party (HP = 0)
        (Class|PaperZDAnimInstance|JumptoNode (Variables|/Script/PaperZD.PaperZDAnimationComponent|GetAnimInstance (Variables|Default|GetAnimationComponent)) "Jump->Downed" "None")
        (else
          ;[0.15 0.15 0.15 0.5] Depleted Enemy (HP = 0), PlayKnockout Anim
          (CallFunction|PlayKnockoutAnim))))))

(fn GetSkillbyIndex
  (params (Index :type Integer))
  (if (or (<= Index -1) (> Index (Utilities|Array|LastIndex (Variables|/Game/_PROJECT_/Data/DataAssets/BattleCharData/PDA_BattleCharData.PDA_BattleCharData_C|GetSkills (Variables|Default|GetBattleCharData)))))
    ;[0.15 0.15 0.15 0.5] BasicAttack
    (return (Variables|/Game/_PROJECT_/Data/DataAssets/BattleCharData/PDA_BattleCharData.PDA_BattleCharData_C|GetBasicAttackData (Variables|Default|GetBattleCharData)))
    (else
      ;[0.15 0.15 0.15 0.5] Skill
      (return (Utilities|Array|Get(acopy) (Variables|/Game/_PROJECT_/Data/DataAssets/BattleCharData/PDA_BattleCharData.PDA_BattleCharData_C|GetSkills (Variables|Default|GetBattleCharData)) Index)))))

(fn PickSkillAnim
  (params (SkillData :type PDA%20Skill%20Data%20Object%20Reference))
  (Utilities|IsValid SkillData
    (:Is%20Valid
      (bind _animation (Variables|/Game/_PROJECT_/Data/DataAssets/SkillData/PDA_SkillData.PDA_SkillData_C|GetAnimation SkillData)
        (:then
          (return _animation))
        (:else
          _)))
    (:Is%20Not%20Valid
      _))
  (return (Variables|/Game/_PROJECT_/Data/DataAssets/BattleCharData/PDA_BattleCharData.PDA_BattleCharData_C|GetAttackAnimDefault (Variables|Default|GetBattleCharData))))