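; Field trigger volume that sends the player into a JRPG battle level when the field player overlaps its box.
; On overlap it has the player store its field position, spawns a refraction Niagara effect at a fixed world location and disables field input through a controller interface.
; After a short delay it plays the transition widget's screen-close animation, waits the global transition delay, then opens the hard-wired dev battle map.
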(event OnComponentBeginOverlap(Box)
  (params (OverlappedComponent :type Primitive%20Component%20Object%20Reference) (OtherActor :type Actor%20Object%20Reference) (OtherComp :type Primitive%20Component%20Object%20Reference) (OtherBodyIndex :type Integer) (bFromSweep :type Boolean) (SweepResult :type Hit%20Result%20Structure%20%28by%20ref%29))
  ;[0.15 0.15 0.15 0.5] Check Field Player
  (bind _asbp_field_player (Utilities|Casting|CastToBP_FieldPlayer OtherActor))
  (Utilities|IsValid _asbp_field_player
    (:Is%20Valid
      ;[0.15 0.15 0.15 0.5] Store field postion and level name
      (Default|StoreFieldPositiononInstance _asbp_field_player)
      ;[0.15 0.15 0.15 0.5] Add Post Process Niagara FX
      (Niagara|SpawnSystematLocation "/Game/Assassin_VFX_Pack/VFX/NS_Post_Process_Refraction.NS_Post_Process_Refraction" "1500.000000,-100.000000,60.000000" "0, 0, 0" "6.000000,6.000000,6.000000")
      ;[0.15 0.15 0.15 0.5] Disable Field Input
      (Class|BPIUIControl|IDisableFieldInput(Message) (Game|GetPlayerController 0))
      ;[0.15 0.15 0.15 0.5] Widget Transition
      (Utilities|FlowControl|RetriggerableDelay 1.5)
      (bind _widgetfield (Class|BPIUIControl|IGetWidgetField(Message) (Game|GetPlayerController 0)))
      (bind _wbp_transition (Variables|/Game/_PROJECT_/Blueprints/Widgets/WBP_Field.WBP_Field_C|GetWBP_Transition _widgetfield)
        (:then
          (Default|PlayScreenCloseAnim _wbp_transition)
          ;[0.15 0.15 0.15 0.5] Open Battle Level
          (Utilities|FlowControl|RetriggerableDelay (Variables|/Game/_PROJECT_/Data/DataAssets/GlobalVariables/PDA_GlobalVariables.PDA_GlobalVariables_C|GetTransitionDelay (CallFunction|GetGlobalVariables)))
          (Game|OpenLevel(byObjectReference) "/Game/_PROJECT_/Map/DevMap_Battle_JRPG.DevMap_Battle_JRPG"))
        (:else)))))

(fn ConstructionScript)