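; Core player controller that manages the field and battle HUD widgets and switches input between gameplay and UI.
; Interface calls create and store each widget, return its reference, toggle UI-only or game-only input with the mouse cursor, and remove the field Enhanced Input mapping context.
; A Q key flip-flop toggles global time dilation between fast and normal game speed.
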(event Input|KeyboardEvents|Q
  (params (Key :type Key%20Structure :default "None"))
  ;[0.15 0.15 0.15 0.5] Set Game Play Fast or Default
  (:Pressed
    (bind _isa (Utilities|FlowControl|FlipFlop)
      (:A
        _)
      (:B
        _))
    (Utilities|Time|SetGlobalTimeDilation (Math|Float|SelectFloat 5.0 1.0 _isa))))

(event EventIDisableFieldInput
  ;[0.15 0.15 0.15 0.5] Disable Field Input
  (CallFunction|DisableFieldInputs))

(event EventIDeactivateUIControls
  ;[0.15 0.15 0.15 0.5] UI Controls
  (CallFunction|DeactivateUIControls))

(event EventIInitWidgetField
  ;[0.15 0.15 0.15 0.5] Init
  (CallFunction|InitWidgetField))

(event EventIInitWidgetBattle
  ;[0.15 0.15 0.15 0.5] Init
  (CallFunction|InitWidgetBattle))

(event EventIActivateUIControls
  (params (WidgetToFocus :type Widget%20Object%20Reference))
  ;[0.15 0.15 0.15 0.5] UI Controls
  (CallFunction|ActivateUIControls WidgetToFocus))

(fn ConstructionScript)

(fn InitWidgetBattle
  (bind _returnvalue (UserInterface|CreateWidget "/Game/_PROJECT_/Blueprints/Widgets/WBP_Battle.WBP_Battle_C" self))
  (bind _output_get (Variables|Default|SetWidgetBattleRef _returnvalue))
  (UserInterface|Viewport|AddtoViewport _output_get 0))

(fn InitWidgetField
  (bind _returnvalue (UserInterface|CreateWidget "/Game/_PROJECT_/Blueprints/Widgets/WBP_Field.WBP_Field_C" self))
  (bind _output_get (Variables|Default|SetWidgetFieldRef _returnvalue))
  (UserInterface|Viewport|AddtoViewport _output_get 0))

(fn ActivateUIControls
  (params (InWidgetToFocus :type Widget%20Object%20Reference))
  ;[0.15 0.15 0.15 0.5] Set InputControll only in UI
  (Input|SetInputModeUIOnly (Game|GetPlayerController 0) InWidgetToFocus "DoNotLock" true)
  ;[0.15 0.15 0.15 0.5] Mouse Cursor
  (Variables|/Script/Engine.PlayerController|SetbShowMouseCursor (Game|GetPlayerController 0) true))

(fn DeactivateUIControls
  (bind _returnvalue (Game|GetPlayerController 0))
  ;[0.15 0.15 0.15 0.5] Set InputControl only in UI
  (Input|SetInputModeGameOnly _returnvalue true)
  ;[0.15 0.15 0.15 0.5] Mouse Cursor
  (Variables|/Script/Engine.PlayerController|SetbShowMouseCursor _returnvalue false))

(fn DisableFieldInputs
  (Input|RemoveMappingContext (PlayerController|LocalPlayerSubsystems|GetEnhancedInputLocalPlayerSubsystem self) "/Game/_PROJECT_/Inputs/Field/IMC_Field.IMC_Field" "(bIgnoreAllPressedKeysUntilRelease=True,bForceImmediately=False,bNotifyUserSettings=False)"))

(fn IGetWidgetBattle
  (return (Variables|Default|GetWidgetBattleRef)))

(fn IGetWidgetField
  (return (Variables|Default|GetWidgetFieldRef)))