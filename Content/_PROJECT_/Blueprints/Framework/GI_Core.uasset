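; GI_Core is the core Game Instance, holding the party's field state and a shared GlobalVariables reference for other systems.
; Interface events write the last field transform and field level name into the PartyFieldAttribute struct.
; Interface getters return that struct and, after a validity check, the GlobalVariables reference, so callers can use both through interfaces.
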(event EventIStoreFieldPosition
  (params (LastFieldTransform :type Transform))
  ;[0.15 0.15 0.15 0.5] Interfaces
  (Utilities|Struct|SetmembersinS_Field (Variables|Game|GetPartyFieldAttribute) LastFieldTransform))

(event EventIFieldLevelName
  (params (FieldLevelName :type String))
  ;[0.15 0.15 0.15 0.5] Interfaces
  (Utilities|Struct|SetmembersinS_Field (Variables|Game|GetPartyFieldAttribute) FieldLevelName))

(fn IGetFieldStruct
  (return (Variables|Game|GetPartyFieldAttribute)))

(fn IGetGlobalVariables
  (bind _globalvariables (Variables|Default|GetGlobalVariables)
    (:then
      (return _globalvariables))
    (:else)))