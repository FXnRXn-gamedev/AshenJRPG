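; GM_Field is the game mode for field maps that spawns and possesses the player pawn on BeginPlay, after focusing the game viewport.
; It reads the field struct from the game instance through an interface message to tell a fresh start from a return from battle.
; An empty stored level name places BP_FieldPlayer at the PlayerStart; otherwise it spawns at the saved last field transform, restoring the player's pre-battle position.
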(event EventBeginPlay
  (Class|WidgetBlueprintLibrary|SetFocustoGameViewport)
  (CallFunction|SpawnPlayer))

(event EventTick
  (params (DeltaSeconds :type Float%20%28single-precision%29)))

(fn ConstructionScript)

(fn SpawnPlayer
  (bind _fieldstruct (Class|BPIInstance|IGetFieldStruct(Message) (Game|GetGameInstance)))
  (if (Utilities|Array|IsEmpty (Utilities|Struct|BreakS_Field _fieldstruct))
    ;[0.15 0.15 0.15 0.5] Start of Game [Not coming from battle Map], Spawn Player at PlayerStart Position
    (bind _returnvalue (Actor|GetActorOfClass "/Script/Engine.PlayerStart"))
    (bind _returnvalue_2 (Game|SpawnActorfromClass "/Game/_PROJECT_/Blueprints/Field/BP_FieldPlayer.BP_FieldPlayer_C" (Math|Transform|MakeTransform (.location (Transformation|GetActorTransform _returnvalue)) (.rotation (Transformation|GetActorTransform _returnvalue)) "1.000000,1.000000,1.000000") "AlwaysSpawn" "MultiplyWithRoot" 0 0))
    (Pawn|Possess (Game|GetPlayerController 0) _returnvalue_2)
    (else
      ;[0.15 0.15 0.15 0.5] Start of Game [Coming from battle Map], Spawn Player at PlayerLast Position
      (bind _fieldstruct_2 (Class|BPIInstance|IGetFieldStruct(Message) (Game|GetGameInstance)))
      (bind _returnvalue_3 (Game|SpawnActorfromClass "/Game/_PROJECT_/Blueprints/Field/BP_FieldPlayer.BP_FieldPlayer_C" (Math|Transform|MakeTransform (.location (Utilities|Struct|BreakS_Field _fieldstruct_2)) (.rotation (Utilities|Struct|BreakS_Field _fieldstruct_2)) "1.000000,1.000000,1.000000") "AlwaysSpawn" "MultiplyWithRoot" 0 0))
      (Pawn|Possess (Game|GetPlayerController 0) _returnvalue_3))))